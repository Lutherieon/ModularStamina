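; Player stamina component that handles Enhanced Input sprinting and one-off action costs, using references and tuning supplied by the owner.
; A looping timer drains stamina during grounded, velocity-detected sprinting, regenerates it below sprint speed, and clears once full.
; Exhaustion stops sprinting, plays a sound once and blocks sprinting until full recovery, with dispatchers broadcasting changes.
; Releasing sprint midair keeps momentum through a polling timer until landing.
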(event Custom|StartStaminaCycle
  ;[0.15 0.15 0.15 0.5] StaminaCycleManager
  (bind _returnvalue (Utilities|Time|SetTimerbyEvent (delegate Custom|StartStaminaCycleManager) 0.1 true))
  (Variables|Timer||SetStaminaTimerHandle _returnvalue))

(event Custom|StartStaminaCycleManager
  ;[0.15 0.15 0.15 0.5] StaminaCycleManager
  (CallFunction|StaminaCycleManager (Variables|Ref|GetCharacter%20Movement%20Comp) (.sprinting (Variables|Ref|GetF%20Character%20Speed))))

(event Custom|EventOnExhaused
  ;[0.15 0.15 0.15 0.5] Exhaustion and Recovery
  (Utilities|FlowControl|Sequence
    (:then_0
      (ActionStateFunction|StopSprinting (Variables|Ref|GetCharacter%20Movement%20Comp)))
    (:then_1
      (Utilities|FlowControl|DoOnce false
        (:Completed
          (Audio|PlaySound2D (Variables|Ref|GetExhaustedSound) 1.0 1.0 0.0 0 0))))))

(event Custom|EventOnStaminaRecovered
  ;[0.15 0.15 0.15 0.5] Exhaustion and Recovery
  (Utilities|FlowControl|DoOnce false) ; enters at Reset
)

(event Custom|ConservationOfMomentum
  ;[0.15 0.15 0.15 0.5] Ziplarken elimizi eger cekersek sprintten yine de momentum korunuyor
  (if (Variables|Boolean|GetbIsSprintingActionActive?)
    ;;[0.15 0.15 0.15 0.5] Zipladi ve sprintinge bastiysa
    (if (not (Class|KismetSystemLibrary|TimerExistsHandle (Variables|Timer|GetConservationOfMomentumHandle)))
      (Variables|/Script/Engine.CharacterMovementComponent|SetMaxWalkSpeed (Variables|Ref|GetCharacter%20Movement%20Comp) (.walking (Variables|Ref|GetF%20Character%20Speed))))
    (else
      ;;[0.15 0.15 0.15 0.5] Zipladi ve sprintingten elini cektiyse
      (if (PureFunction|BIsPlayerGrounded? (Variables|Ref|GetCharacter%20Movement%20Comp))
        (Variables|/Script/Engine.CharacterMovementComponent|SetMaxWalkSpeed (Variables|Ref|GetCharacter%20Movement%20Comp) (.walking (Variables|Ref|GetF%20Character%20Speed)))
        (Utilities|Time|ClearandInvalidateTimerbyHandle (Variables|Timer|GetConservationOfMomentumHandle))))))

(event Input|EnhancedActionEvents|EnhancedInputActionIA_Sprinting
  (params (ActionValue :type Boolean) (ElapsedSeconds :type Float%20%28double-precision%29) (TriggeredSeconds :type Float%20%28double-precision%29) (InputAction :type Input%20Action%20Object%20Reference :default "/Game/Blueprint/StaminaSystem/Input/Action/IA_Sprinting.IA_Sprinting"))
  (bind _character_movement_comp (Variables|Ref|GetCharacter%20Movement%20Comp))
  ;[0.15 0.15 0.15 0.5] Start - Stop | and momentum stabilitesi
  (:Started
    (ActionStateFunction|StartSprinting _character_movement_comp))
  (:Completed
    (ActionStateFunction|StopSprinting _character_movement_comp)))

(event EventBeginPlay
  ;[0.15 0.15 0.15 0.5] Add mapping context for sprinting action
  (Input|AddMappingContext (PlayerController|LocalPlayerSubsystems|GetEnhancedInputLocalPlayerSubsystem (Game|GetPlayerController 0)) "/Game/Blueprint/StaminaSystem/Input/IMC_Sprinting.IMC_Sprinting" 0 "(bIgnoreAllPressedKeysUntilRelease=True,bForceImmediately=False,bNotifyUserSettings=False)"))

(event EventGetMovementReferences
  (params (Player :type Actor%20Object%20Reference) (CharacterMovement :type Character%20Movement%20Component%20Object%20Reference) (F_CharacterSpeed :type F%20Character%20Speed%20Structure) (MaxStamina :type Float%20%28double-precision%29) (ExhaustedSound :type Sound%20Base%20Object%20Reference) (DrainAmount :type Float%20%28double-precision%29) (RegenAmount :type Float%20%28double-precision%29))
  ;[0.15 0.15 0.15 0.5] Setup Initilize References For Component - Player must be give the data
  (Variables|Default|SetPlayer Player)
  (bind _output_get (Variables|Ref|SetCharacter%20Movement%20Comp CharacterMovement))
  (bind _output_get_2 (Variables|Ref|SetF%20Character%20Speed F_CharacterSpeed))
  (Variables|/Script/Engine.CharacterMovementComponent|SetMaxWalkSpeed _output_get (.walking _output_get_2))
  (Variables|Ref||SetMax%20Stamina MaxStamina)
  (Variables|Ref|SetCurrentStamina MaxStamina)
  (Variables|Ref|SetExhaustedSound ExhaustedSound)
  (Variables|Ref|SetDrainAmount DrainAmount)
  (Variables|Ref|SetRegenAmount RegenAmount))

(event EventNotifyOneTimeAction
  (params (bIsPlayerPerformedAction? :type Boolean) (CurrentState :type E_CharacterState%20Enum :default "NewEnumerator0") (OneTimeDrainAmountRef :type Float%20%28double-precision%29))
  ;[0.15 0.15 0.15 0.5] Jumping Roll gibi actionlarda stamina drain
  (Variables|Default|SetOne%20Time%20Drain%20Amount%20Ref OneTimeDrainAmountRef)
  (Variables|Default|SetCharacter%20State%20Ref CurrentState)
  (bind _output_get (Variables|Boolean|SetbIsPlayerPerformedActionRef? bIsPlayerPerformedAction?))
  (if (and _output_get (not (Variables|Boolean||GetbIsExhausted?)))
    (if (and (PureFunction|BIsPlayerGrounded? (Variables|Ref|GetCharacter%20Movement%20Comp)) (PureFunction|BIsPlayerSprinting? (Variables|Ref|GetCharacter%20Movement%20Comp) (.sprinting (Variables|Ref|GetF%20Character%20Speed))))
      (ActionStateFunction|DrainStamina true (Variables|Default|GetOne%20Time%20Drain%20Amount%20Ref))
      (CallFunction|StartStaminaCycle)
      (elif (Utilities|Enum|NotEqual(Enum) (Variables|Default|GetCharacter%20State%20Ref) "NewEnumerator2")
        (ActionStateFunction|DrainStamina true (Variables|Default|GetOne%20Time%20Drain%20Amount%20Ref))
        (CallFunction|StartStaminaCycle)))))

(event EventTick
  (params (DeltaSeconds :type Float%20%28single-precision%29)))

(fn StartSprinting
  (params (CharacterMovementComponent :type Character%20Movement%20Component%20Object%20Reference))
  (Variables|Boolean|SetbIsSprintingActionActive? true)
  (if (and (not (Variables|Boolean||GetbIsExhausted?)) (PureFunction|BIsPlayerGrounded? CharacterMovementComponent))
    (Variables|/Script/Engine.CharacterMovementComponent|SetMaxWalkSpeed (Variables|Ref|GetCharacter%20Movement%20Comp) (.sprinting (Variables|Ref|GetF%20Character%20Speed)))
    (CallFunction|StartStaminaCycle)
    (elif (not (PureFunction|BIsPlayerGrounded? CharacterMovementComponent))
      (CallFunction|ConservationOfMomentum))))

(fn StopSprinting
  (params (CharacterMovementComponent :type Character%20Movement%20Component%20Object%20Reference))
  (Variables|Boolean|SetbIsSprintingActionActive? false)
  (if (PureFunction|BIsPlayerGrounded? CharacterMovementComponent)
    ;[0.15 0.15 0.15 0.5] Yerdeyken Stoplarsa
    (Variables|/Script/Engine.CharacterMovementComponent|SetMaxWalkSpeed (Variables|Ref|GetCharacter%20Movement%20Comp) (.walking (Variables|Ref|GetF%20Character%20Speed)))
    (else
      (bind _returnvalue (Utilities|Time|SetTimerbyEvent (EventDispatchers|CreateEvent :!event Custom|ConservationOfMomentum) 0.1 true))
      (Variables|Timer|SetConservationOfMomentumHandle _returnvalue))))

(fn StaminaCycleManager
  (params (CharacterMovementComponent :type Character%20Movement%20Component%20Object%20Reference) (SprintingSpeedRef :type Float%20%28double-precision%29))
  (Utilities|CheckPlayerStateIsAvaibleforDrainorRegen CharacterMovementComponent SprintingSpeedRef
    (:StaminaDrain
      (ActionStateFunction|DrainStamina false 0.0)
      (if (not (PureFunction|BIsStaminaFull?))
        (Variables|Boolean|SetbIsDrainCycleStarted? true)
        (if (PureFunction|BIsPlayerExhausted?)
          (Variables|Boolean||SetbIsExhausted? true)
          (CallFunction|EventonExhaused)
          (Default|CallOnExhaustedState))))
    (:StaminaRegen
      (ActionStateFunction|RegenStamina)
      (if (and (PureFunction|BIsStaminaFull?) (not (PureFunction|BIsPlayerSprinting? CharacterMovementComponent SprintingSpeedRef)))
        (Variables|Boolean||SetbIsExhausted? false)
        (CallFunction|EventonStaminaRecovered)
        (Default|CallOnStaminaRecovered)
        (if (and (PureFunction|BIsStaminaFull?) (Variables|Boolean|GetbIsDrainCycleStarted?))
          (Utilities|Time|ClearandInvalidateTimerbyHandle (Variables|Timer||GetStaminaTimerHandle))
          (Variables|Boolean|SetbIsDrainCycleStarted? false))))))

(fn BIsPlayerSprinting?
  (params (CharacterMovementComponent :type Character%20Movement%20Component%20Object%20Reference) (SprintingSpeedRef :type Float%20%28double-precision%29))
  ;[0.15 0.15 0.15 0.5] Playerin Kosup Kosmadigini Hiz bakimindan kontrol ediyoruz. bIsSprintingActive? tus olarak oldugu icin batigi surece hep dogru gelecek ancak burada ya da stun oldugunda sprinte bassak bile hizimiz 0 olacagi icin bu false olacak
  (return (> (Math|Vector|VectorLength (Pawn|Components|CharacterMovement|GetLastUpdateVelocity CharacterMovementComponent)) (- SprintingSpeedRef 5.0))))

(fn BIsPlayerGrounded?
  (params (CharacterMovementComponent :type Character%20Movement%20Component%20Object%20Reference))
  ;[0.15 0.15 0.15 0.5] Playerin son hizini 0la 1 arasina aliyoruz ve Z duzleminde bakiyoruz. Eger 0sa yere basiyordur.
  (Utilities|IsValid CharacterMovementComponent
    (:Is%20Valid
      (return (== (.z (Math|Vector|Normalize (Pawn|Components|CharacterMovement|GetLastUpdateVelocity CharacterMovementComponent))) 0.0)))))

(fn DrainStamina
  (params (bIsOneShotDrain? :type Boolean) (OneShotDrainAmount :type Float%20%28double-precision%29))
  (bind _output_get (Variables|Ref|SetCurrentStamina (Math|Float|Clamp(Float) (- (Variables|Ref|GetCurrentStamina) (Math|Float|SelectFloat OneShotDrainAmount (Variables|Ref|GetDrainAmount) bIsOneShotDrain?)) 0.0 (Variables|Ref||GetMax%20Stamina))))
  (Default|CallOnUpdateStamina (.StaminaText (CallFunction|GetStaminaPercentage _output_get)) (.StaminaPercentage (CallFunction|GetStaminaPercentage _output_get)))
  (return))

(fn GetStaminaPercentage
  (params (RawStamina :type Float%20%28double-precision%29))
  (bind _max_stamina (Variables|Ref||GetMax%20Stamina))
  (bind _returnvalue (/ RawStamina _max_stamina))
  (return (Utilities|Text|ToText(Float) (* _returnvalue 1e+02) "HalfToEven") _returnvalue))

(fn BIsStaminaFull?
  (return (== (Variables|Ref|GetCurrentStamina) (Variables|Ref||GetMax%20Stamina))))

(fn BIsPlayerExhausted?
  (return (<= (Variables|Ref|GetCurrentStamina) 0.0)))

(fn RegenStamina
  (bind _output_get (Variables|Ref|SetCurrentStamina (Math|Float|Clamp(Float) (+ (Variables|Ref|GetCurrentStamina) (Variables|Ref|GetRegenAmount)) 0.0 (Variables|Ref||GetMax%20Stamina))))
  (Default|CallOnUpdateStamina (.StaminaText (CallFunction|GetStaminaPercentage _output_get)) (.StaminaPercentage (CallFunction|GetStaminaPercentage _output_get)))
  (return))

(fn BIsPlayerPressMoveActions?
  (params (Character%20Movement%20Comp :type Character%20Movement%20Component%20Object%20Reference))
  (return (> (Math|Vector|VectorLength (Pawn|Components|CharacterMovement|GetCurrentAcceleration Character%20Movement%20Comp)) 0.0)))

(fn BIsPlayerPerformingandAction?)