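; Grapple hook component for the third-person character that picks and highlights the best grapple target, with only the targeting stage implemented.
; Tick dispatches on GrappleState; Firing, Near Target and Hit are empty stubs.
; Inactive sphere-overlaps target actors in range, keeps the line-of-sight one closest to camera forward within an angle cutoff, and prints its name.
; Activation switches between old and new targets only when the selection changes.
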(event EventBeginPlay
  (bind _asbp_third_person_character (Utilities|Casting|CastToBP_ThirdPersonCharacter (Components|GetOwner)))
  (Variables|Private|SetOwningCharacter _asbp_third_person_character))

(event EventTick
  (params (DeltaSeconds :type Float%20%28single-precision%29))
  (switch Utilities|FlowControl|Switch|SwitchonE_GrappleHookState (Variables|Private|GetGrappleState)
    (:NewEnumerator0
      (Private|Inactive))
    (:NewEnumerator1
      (Private|Firing))
    (:NewEnumerator2
      (Private|NearTarget))
    (:NewEnumerator3
      (Private|HitTarget))))

(fn Inactive
  (bind _outactors (Collision|SphereOverlapActors (Transformation|GetActorLocation (Variables|Private|GetOwningCharacter)) (Variables|Private|GetMaxGrappleDistance) (Utilities|Array|MakeArray "ObjectTypeQuery1") "/Game/Blueprint/GrappleHookSystem/BP_GrappleHookTarget.BP_GrappleHookTarget_C"))
  (bind _besttarget (Private|FindBestGrappleTarget _outactors))
  (Private|SetCurrentTargetVisibility (.AsBP%20Grapple%20Hook%20Target (Utilities|Casting|CastToBP_GrappleHookTarget _besttarget)))
  (Development|PrintString (Utilities|GetDisplayName (.AsBP%20Grapple%20Hook%20Target (Utilities|Casting|CastToBP_GrappleHookTarget _besttarget)))))

(fn Firing)

(fn NearTarget)

(fn HitTarget)

(fn FindBestGrappleTarget
  (params (Targets :type Array%20of%20Actor%20Object%20References))
  (bind _owningcharacter (Variables|Private|GetOwningCharacter))
  (for _array_element Targets
    (LocalVariables|SetCurrentTarget%28Local%29 _array_element)
    (bind _outhit (Collision|LineTraceByChannel (Transformation|GetActorLocation (Variables|Private|GetOwningCharacter)) (Transformation|GetActorLocation (LocalVariables|GetCurrentTarget%28Local%29)) "TraceTypeQuery1" false (Utilities|Array|MakeArray (Variables|Private|GetOwningCharacter)) "None" true "(R=1.000000,G=0.000000,B=0.000000,A=1.000000)" "(R=0.000000,G=1.000000,B=0.000000,A=1.000000)" 1.0))
    (if (== (.HitActor (Collision|BreakHitResult _outhit)) (LocalVariables|GetCurrentTarget%28Local%29))
      (Utilities|FlowControl|Sequence
        (:then_0
          ;[0.15 0.15 0.15 0.5] (Step 1)Calculate Angles to Target
          (LocalVariables|SetCurrentAngle%28Local%29 (Class|KismetMathLibrary|DegAcos (Math|Vector|DotProduct (Math|Vector|Normalize (- (Transformation|GetActorLocation (LocalVariables|GetCurrentTarget%28Local%29)) (Transformation|GetActorLocation _owningcharacter))) (Math|Vector|GetForwardVector (Variables|/Game/Blueprint/Core/Player/BP_ThirdPersonCharacter.BP_ThirdPersonCharacter_C|GetFollowCamera _owningcharacter))))))
        (:then_1
          ;[0.15 0.15 0.15 0.5] (Step 2) if the angle is less than the current angle or there is no best target, make this the next target
          (if (or (< (LocalVariables|GetCurrentAngle%28Local%29) (LocalVariables|GetBestAngle%28Local%29)) (not (Utilities|IsValid (LocalVariables|GetBestTarget%28Local%29))))
            (LocalVariables|SetBestTarget%28Local%29 (LocalVariables|GetCurrentTarget%28Local%29))
            (LocalVariables|SetBestAngle%28Local%29 (LocalVariables|GetCurrentAngle%28Local%29))))
        (:then_2
          ;[0.15 0.15 0.15 0.5] Histerezis" (Hysteresis)
          (if (not (< (LocalVariables|GetBestAngle%28Local%29) 8e+01))
            (LocalVariables|SetBestTarget%28Local%29 0))))))
  ;[0.15 0.15 0.15 0.5] Return
  (return (LocalVariables|GetBestTarget%28Local%29)))

(fn SetCurrentTargetVisibility
  (params (NewTarget :type BP%20Grapple%20Hook%20Target%20Object%20Reference))
  (if (!= NewTarget (Variables|Private|GetCurrentTarget))
    (Utilities|FlowControl|Sequence
      (:then_0
        ;[0.15 0.15 0.15 0.5] Hide Old Target
        (bind _currenttarget (Variables|Private|GetCurrentTarget)
          (:then
            (Default|SetActive _currenttarget false))
          (:else)))
      (:then_1
        ;[0.15 0.15 0.15 0.5] Set New Target
        (Variables|Private|SetCurrentTarget NewTarget))
      (:then_2
        ;[0.15 0.15 0.15 0.5] Show new Target
        (bind _currenttarget_2 (Variables|Private|GetCurrentTarget)
          (:then
            (Default|SetActive _currenttarget_2 true))
          (:else))))))